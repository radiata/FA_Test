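; BP_ItemRenderer renders an inventory item's mesh through a SceneCaptureComponent2D, with rotation and zoom control.
; UpdateStaticMesh applies a valid mesh, camera position and zoom limits from the item's renderer settings, while ResetMesh clears the mesh.
; RotateMesh turns scaled input deltas into local rotation.
; SetZoom moves the capture along X within the limits, tracking CurrentZoom, which is seeded at construction and not resynced on item change.
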(fn ConstructionScript
  (Variables|Default|SetCurrent%20Zoom (.X (Math|Vector|BreakVector (Variables|/Script/Engine.SceneComponent|GetRelativeLocation (Variables|Default|GetSceneCaptureComponent2D))))))

(fn UpdateStaticMesh
  (params (Item%20Renderer%20Settings :type S%20Item%20Renderer%20Settings%20Structure))
  (bind (_mesh _cameraposition _maxposition _minposition) (Utilities|Struct|BreakS_ItemRendererSettings Item%20Renderer%20Settings))
  (if (!= _mesh 0)
    (Components|StaticMesh|SetStaticMesh (Variables|Default|GetStaticMesh) _mesh)
    (Transformation|SetRelativeLocation (Variables|Default|GetSceneCaptureComponent2D) _cameraposition false false)
    (CallFunction|UpdatePosition _maxposition _minposition)))

(fn UpdatePosition
  (params (Max%20Position :type Float%20%28double-precision%29) (Min%20Position :type Float%20%28double-precision%29))
  (Variables|Default|SetMax%20Position Max%20Position)
  (Variables|Default|SetMin%20Position Min%20Position))

(fn ResetMesh
  (Components|StaticMesh|SetStaticMesh (Variables|Default|GetStaticMesh) 0))

(fn RotateMesh
  (params (X_Delta :type Float%20%28double-precision%29) (Y_Delta :type Float%20%28double-precision%29))
  (bind _rotation_multiplier (Variables|Default|GetRotation%20Multiplier))
  (Transformation|AddLocalRotation (Variables|Default|GetStaticMesh) (Math|Rotator|MakeRotator (* X_Delta _rotation_multiplier) (* Y_Delta _rotation_multiplier) 0.0) false false))

(fn SetZoom
  (params (Zoom%20Delta :type Float%20%28double-precision%29))
  (bind _scenecapturecomponent2d (Variables|Default|GetSceneCaptureComponent2D))
  (bind _returnvalue (Transformation|GetRelativeTransform _scenecapturecomponent2d))
  (bind (_location _rotation _scale) (Math|Transform|BreakTransform _returnvalue))
  (bind (_x _y _z) (Math|Vector|BreakVector _location))
  (Transformation|SetRelativeTransform (Variables|Default|GetSceneCaptureComponent2D) (Math|Transform|MakeTransform (Math|Vector|MakeVector (Math|Float|Clamp(Float) (+ (Variables|Default|GetCurrent%20Zoom) (* Zoom%20Delta (Variables|Default|GetZoom%20Multiplier))) (Variables|Default|GetMin%20Position) (Variables|Default|GetMax%20Position)) _y _z) _rotation _scale) false false)
  (Variables|Default|SetCurrent%20Zoom (Math|Float|Clamp(Float) (+ (Variables|Default|GetCurrent%20Zoom) (* Zoom%20Delta (Variables|Default|GetZoom%20Multiplier))) (Variables|Default|GetMin%20Position) (Variables|Default|GetMax%20Position))))